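; Interactive hinged door for a Layer of Fear project that swings in response to a movement value passed to its Interact event.
; Interact scales that value by Sensitivity, clamps it per call and adds it to the door mesh's relative yaw.
; An inverted ClampAngle comparison detects yaw leaving the 0–90 degree swing, snapping it just inside fully open or to closed.
; The IsClosed flag lets movement resume from the closed position.
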(event `/Game/LayerOfFear/BPI_Interact.Interact`
  (params (Movement :type "Float (double-precision)"))
  (bind _sm_door (`self.SM_Door`))
  (bind (_relativerotation_roll _relativerotation_pitch _relativerotation_yaw) (`KismetMathLibrary.BreakRotator` (`SceneComponent.RelativeRotation` (`self.SM_Door`))))
  (if (or (not (== _relativerotation_yaw (`KismetMathLibrary.ClampAngle` _relativerotation_yaw 90.0 0.0))) (`self.IsClosed`))
    (set `self.IsClosed` false)
    (`SceneComponent.K2_AddRelativeRotation` _sm_door (`KismetMathLibrary.MakeRotator` 0.0 0.0 (`KismetMathLibrary.FClamp` (* Movement (`self.Sensitivity`)) -10.0 10.0)) false false)
    (elif (>= _relativerotation_yaw 90.0)
      (`SceneComponent.K2_SetRelativeRotation` _sm_door (struct :`Yaw` 89.9) false false)
      (else
        (`SceneComponent.K2_SetRelativeRotation` _sm_door (struct) false false)
        (set `self.IsClosed` true)))))

(fn `UserConstructionScript`)